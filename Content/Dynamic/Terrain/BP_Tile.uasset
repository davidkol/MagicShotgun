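; BP_Tile is one segment of an infinite terrain that scatters containers, rocks and other props on BeginPlay through PlaceActors.
; The player entering LockingVolume opens the green barrier; leaving it locks the barrier red and tells InfiniteTerrainGameMode to spawn another tile.
; GetAttachLocation exposes the Arrow's transform as an attach point.
; The tile destroys itself when the player overlaps DestructingVolume.
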(event `self.ReceiveBeginPlay`
  (`self.PlaceActors` "/Game/Dynamic/Terrain/Props/BP_Container.BP_Container_C" 1 1 400.0 1.0 1.0)
  (`self.PlaceActors` "/Game/Dynamic/Terrain/Props/BP_Canister.BP_Canister_C" 1 5 50.0 1.0 1.0)
  (`self.PlaceActors` "/Game/Dynamic/Terrain/Props/BP_Rock01.BP_Rock01_C" 1 3 150.0 1.0 5.0)
  (`self.PlaceActors` "/Game/Dynamic/Terrain/Props/BP_Rock02.BP_Rock02_C" 1 2 250.0 1.0 5.0)
  (`self.PlaceActors` "/Game/Dynamic/Terrain/Props/BP_Rock03.BP_Rock03_C" 0 1 250.0 8.0 12.0)
  (`self.PlaceActors` "/Game/Dynamic/Terrain/Props/BP_Sack.BP_Sack_C" 1 3 250.0 1.0 1.0)
  (`self.PlaceActors` "/Game/Dynamic/Terrain/Props/BP_Box.BP_Box_C" 1 5 100.0 1.0 1.0))

(event `self.Locking Volume.OnComponentBeginOverlap`
  (params (OverlappedComponent :type "PrimitiveComponent Object Reference") (OtherActor :type "Actor Object Reference") (OtherComp :type "PrimitiveComponent Object Reference") (OtherBodyIndex :type Integer) (bFromSweep :type Boolean) (SweepResult :type "HitResult Structure (by ref)"))
  (`self.Is Player Character` OtherActor)
  (`self.Unlock Barrier`))

(event `self.Locking Volume.OnComponentEndOverlap`
  (params (OverlappedComponent :type "PrimitiveComponent Object Reference") (OtherActor :type "Actor Object Reference") (OtherComp :type "PrimitiveComponent Object Reference") (OtherBodyIndex :type Integer))
  (`self.Is Player Character` OtherActor)
  (`self.Lock Barrier`)
  (bind _asinfinite_terrain_game_mode (cast `/Game/Dynamic/InfiniteTerrainGameMode` (`GameplayStatics.GetGameMode`)))
  (`/Game/Dynamic/InfiniteTerrainGameMode.Spawn Tile` _asinfinite_terrain_game_mode))

(event `self.Destructing Volume.OnComponentBeginOverlap`
  (params (OverlappedComponent :type "PrimitiveComponent Object Reference") (OtherActor :type "Actor Object Reference") (OtherComp :type "PrimitiveComponent Object Reference") (OtherBodyIndex :type Integer) (bFromSweep :type Boolean) (SweepResult :type "HitResult Structure (by ref)"))
  (`self.Is Player Character` OtherActor)
  (`self.K2_DestroyActor`))

(fn `Get Attach Location`
  (returns (`Attach Transform` :type "Transform Structure"))
  (return (`SceneComponent.K2_GetComponentToWorld` (`self.Arrow`))))

(fn `Lock Barrier`
  (bind _barrier (`self.Barrier`))
  (`PrimitiveComponent.SetCollisionEnabled` _barrier "QueryAndPhysics")
  (`PrimitiveComponent.SetMaterial` _barrier 0 "/Game/Dynamic/Terrain/MI_Barrier_Red.MI_Barrier_Red"))

(fn `Unlock Barrier`
  (bind _barrier (`self.Barrier`))
  (`PrimitiveComponent.SetCollisionEnabled` _barrier "NoCollision")
  (`PrimitiveComponent.SetMaterial` _barrier 0 "/Game/Dynamic/Terrain/MI_Barrier_Green.MI_Barrier_Green"))

(fn `UserConstructionScript`)