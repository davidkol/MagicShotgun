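; BP_EnemyContext is an EQS context that supplies the enemy's target player as the single actor for environment queries.
; For an AI querier, it returns the EnemyPlayer stored on its BP_EnemyAIController.
; For a BP_EQSTester querier, it returns the first BP_PlayerCharacter found in the world, so queries can be previewed without an AI controller.
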(fn `ProvideSingleActor`
  (params (QuerierObject :type "Object Object Reference") (QuerierActor :type "Actor Object Reference"))
  (returns (ResultingActor :type "Actor Object Reference"))
  (locals (TempEnemy :type "/Game/Dynamic/Character/Behavior/BP_PlayerCharacter Object Reference"))
  (bind _returnvalue (`AIBlueprintHelperLibrary.GetAIController` QuerierActor))
  (cast `/Game/Dynamic/Character/Behavior/Enemy/BP_EQSTester` QuerierActor
    (:`then`
      (bind _outactors (`GameplayStatics.GetAllActorsOfClass` "/Game/Dynamic/Character/Behavior/BP_PlayerCharacter.BP_PlayerCharacter_C"))
      (bind _output_get (set `local.TempEnemy` (`|GetArrayItem` _outactors)))
      (return _output_get))
    (:`CastFailed`
      (if (!= _returnvalue null)
        (bind _asbp_enemy_aicontroller (cast `/Game/Dynamic/Character/Behavior/Enemy/BP_EnemyAIController` _returnvalue))
        (set `local.TempEnemy` (`/Game/Dynamic/Character/Behavior/Enemy/BP_EnemyAIController.EnemyPlayer` _asbp_enemy_aicontroller))
        (return _output_get)))))