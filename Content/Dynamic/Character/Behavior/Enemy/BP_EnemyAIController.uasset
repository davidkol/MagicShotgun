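; AI controller for enemy characters that runs the BT_Enemy behavior tree and tracks the player.
; BeginPlay stores the player character and writes it to the EnemyPlayer blackboard key.
; AI perception updates involving the player set or clear focus on them, based only on the first last-sensed stimulus.
; Distance-based logic for the pawn's Swinging flag and the WithinRunningDistance key is present but disconnected, and Tick is empty.
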(event `self.ReceiveBeginPlay`
  (`self.RunBehaviorTree` "/Game/Dynamic/Character/Behavior/Enemy/BT_Enemy.BT_Enemy")
  (bind _asbp_player_character (cast `/Game/Dynamic/Character/Behavior/BP_PlayerCharacter` (`GameplayStatics.GetPlayerCharacter` 0)))
  (bind _output_get (set `self.EnemyPlayer` _asbp_player_character))
  (`BlackboardComponent.SetValueAsObject` (`AIBlueprintHelperLibrary.GetBlackboard` null) "EnemyPlayer" _output_get))

(event `self.AIPerception.OnPerceptionUpdated`
  (params (UpdatedActors :type "Array of Actor Object Reference"))
  (bind _enemyplayer (`self.EnemyPlayer`))
  (for _array_element UpdatedActors
    (if (== _array_element _enemyplayer)
      (`self.Update Enemy Sensed` _enemyplayer))))

(event `self.ReceiveTick`
  (params (DeltaSeconds :type "Float (single-precision)")))

(fn `Update Enemy Sensed`
  (params (Enemy :type "Actor Object Reference"))
  (bind _info (`AIPerceptionComponent.GetActorsPerception` (`self.AIPerception`) Enemy))
  (bind (_output_age _output_expirationage _output_strength _output_stimuluslocation _output_receiverlocation _output_tag _output_bsuccessfullysensed) (break `AIStimulus` (`|GetArrayItem` (`.LastSensedStimuli` (break `ActorPerceptionBlueprintInfo` _info)))))
  (if _output_bsuccessfullysensed
    (`self.K2_SetFocus` Enemy)
    (else
      (`self.K2_ClearFocus`))))

(fn `UserConstructionScript`)