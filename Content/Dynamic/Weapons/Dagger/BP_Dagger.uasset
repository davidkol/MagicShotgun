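; BP_Dagger is a melee weapon Blueprint for a dagger that stabs enemy characters.
; Damage applies a fixed amount to the first BP_EnemyCharacter overlapping the MeleeWeapon component and prints its name.
; PlayAnim plays the stab animation on that component, and GetSpeedCo exposes the weapon's speed coefficient.
; An overlap event on Melee_Weapon only prints the other actor's name, with no damage.
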(event `self.Melee_Weapon.OnComponentBeginOverlap`
  (params (OverlappedComponent :type "PrimitiveComponent Object Reference") (OtherActor :type "Actor Object Reference") (OtherComp :type "PrimitiveComponent Object Reference") (OtherBodyIndex :type Integer) (bFromSweep :type Boolean) (SweepResult :type "HitResult Structure (by ref)"))
  (`KismetSystemLibrary.PrintString` (`KismetSystemLibrary.GetDisplayName` OtherActor)))

(fn `Damage`
  (bind _output (`|GetArrayItem` (`PrimitiveComponent.GetOverlappingActors` (`self.Melee_Weapon`) "/Game/Dynamic/Character/Behavior/BP_EnemyCharacter.BP_EnemyCharacter_C")))
  (if (`KismetSystemLibrary.IsValid` _output)
    (`GameplayStatics.ApplyDamage` _output 5.0)
    (`KismetSystemLibrary.PrintString` (`KismetSystemLibrary.GetDisplayName` _output))))

(fn `GetSpeedCo`
  (returns (SpeedCo :type "Float (double-precision)"))
  (return (`self.SpeedCoefficiant`)))

(fn `PlayAnim`
  (`SkeletalMeshComponent.PlayAnimation` (`self.Melee_Weapon`) "/Game/Dynamic/Weapons/Dagger/Animations/A_Dagger_Stab.A_Dagger_Stab" false))

(fn `UserConstructionScript`)