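; BP_Spear is a spear weapon that can strike in melee or be thrown, ignoring overlaps with the player character.
; Melee overlaps during animation clear the thrown state and call ReduceDurability with a zero amount, destroying the spear if durability is depleted.
; A thrown spear's Box overlap spawns two BP_SpearDamage actors once, then destroys it.
; Damage hits the first overlapping enemy, while PlayThrow is empty, with disconnected radial-force debug logic.
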(event `self.Melee_Weapon.OnComponentBeginOverlap`
  (params (OverlappedComponent :type "PrimitiveComponent Object Reference") (OtherActor :type "Actor Object Reference") (OtherComp :type "PrimitiveComponent Object Reference") (OtherBodyIndex :type Integer) (bFromSweep :type Boolean) (SweepResult :type "HitResult Structure (by ref)"))
  (if (== (`GameplayStatics.GetObjectClass` OtherActor) "/Game/Dynamic/Character/Behavior/BP_PlayerCharacter.BP_PlayerCharacter_C")
    _
    (elif (`SkeletalMeshComponent.IsPlaying` (`self.Melee_Weapon`))
      (`self.ReduceDurability` 0.0)
      (`self.SetThrownStatus` false)
      (bind _returnvalue (`self.GetDurability`))
      (if (<= _returnvalue 0.0)
        (`self.K2_DestroyActor`)))))

(event `self.Box.OnComponentBeginOverlap`
  (params (OverlappedComponent :type "PrimitiveComponent Object Reference") (OtherActor :type "Actor Object Reference") (OtherComp :type "PrimitiveComponent Object Reference") (OtherBodyIndex :type Integer) (bFromSweep :type Boolean) (SweepResult :type "HitResult Structure (by ref)"))
  (bind _returnvalue (`self.GetTransform`))
  (if (not (== (`GameplayStatics.GetObjectClass` OtherActor) "/Game/Dynamic/Character/Behavior/BP_PlayerCharacter.BP_PlayerCharacter_C"))
    (bind _returnvalue_2 (`self.GetThrownStatus`))
    (if _returnvalue_2
      (`/Engine/EditorBlueprintResources/StandardMacros.DoOnce` false
        (:`Completed`
          (`|SpawnActorFromClass` "/Game/Dynamic/Weapons/Spear/BP_SpearDamage.BP_SpearDamage_C" _returnvalue "Undefined" "OverrideRootScale" null null)
          (`|SpawnActorFromClass` "/Game/Dynamic/Weapons/Spear/BP_SpearDamage.BP_SpearDamage_C" _returnvalue "Undefined" "OverrideRootScale" null null)
          (`self.K2_DestroyActor`))))))

(fn `Damage`
  (bind _output (`|GetArrayItem` (`PrimitiveComponent.GetOverlappingActors` (`self.Melee_Weapon`) "/Game/Dynamic/Character/Behavior/Enemy/BP_EnemyCharacter.BP_EnemyCharacter_C")))
  (if (`KismetSystemLibrary.IsValid` _output)
    (`GameplayStatics.ApplyDamage` _output 5.0)))

(fn `GetSpeedCo`
  (returns (SpeedCo :type "Float (double-precision)"))
  (return 0.0))

(fn `Play Anim`
  (`SkeletalMeshComponent.PlayAnimation` (`self.Melee_Weapon`) null false))

(fn `PlayThrow`)

(fn `UserConstructionScript`)