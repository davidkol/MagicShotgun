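; Sword weapon that swings in melee and breaks into damage actors when thrown.
; Damage applies a fixed hit to the first enemy overlapping the weapon mesh, while PlayAnim plays the swing animation.
; When thrown, a box overlap with any non-player actor spawns two BP_SwordDamage actors once, then destroys the sword.
; Mesh overlap and destruction events only print debug text, and GetSpeedCo returns zero.
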(event `self.Melee_Weapon.OnComponentBeginOverlap`
  (params (OverlappedComponent :type "PrimitiveComponent Object Reference") (OtherActor :type "Actor Object Reference") (OtherComp :type "PrimitiveComponent Object Reference") (OtherBodyIndex :type Integer) (bFromSweep :type Boolean) (SweepResult :type "HitResult Structure (by ref)"))
  (`KismetSystemLibrary.PrintString` (`KismetSystemLibrary.GetDisplayName` OtherActor)))

(event `self.ReceiveTick`
  (params (DeltaSeconds :type "Float (single-precision)")))

(event `self.ReceiveDestroyed`
  (`KismetSystemLibrary.PrintString` (`KismetStringLibrary.Conv_VectorToString` (`SceneComponent.K2_GetComponentLocation` (`self.Melee_Weapon`))) true true (struct :`G` 0.66 :`B` 1.0 :`A` 1.0) 0.1))

(event `self.Box.OnComponentBeginOverlap`
  (params (OverlappedComponent :type "PrimitiveComponent Object Reference") (OtherActor :type "Actor Object Reference") (OtherComp :type "PrimitiveComponent Object Reference") (OtherBodyIndex :type Integer) (bFromSweep :type Boolean) (SweepResult :type "HitResult Structure (by ref)"))
  (bind _returnvalue (`self.GetTransform`))
  (if (not (== (`GameplayStatics.GetObjectClass` OtherActor) "/Game/Dynamic/Character/Behavior/BP_PlayerCharacter.BP_PlayerCharacter_C"))
    (bind _returnvalue_2 (`self.GetThrownStatus`))
    (if _returnvalue_2
      (`/Engine/EditorBlueprintResources/StandardMacros.DoOnce` false
        (:`Completed`
          (`|SpawnActorFromClass` "/Game/Dynamic/Weapons/Sword/BP_SwordDamage.BP_SwordDamage_C" _returnvalue "Undefined" "OverrideRootScale" null null)
          (`|SpawnActorFromClass` "/Game/Dynamic/Weapons/Sword/BP_SwordDamage.BP_SwordDamage_C" _returnvalue "Undefined" "OverrideRootScale" null null)
          (`self.K2_DestroyActor`))))))

(fn `Damage`
  (bind _output (`|GetArrayItem` (`PrimitiveComponent.GetOverlappingActors` (`self.Melee_Weapon`) "/Game/Dynamic/Character/Behavior/BP_EnemyCharacter.BP_EnemyCharacter_C")))
  (if (`KismetSystemLibrary.IsValid` _output)
    (`GameplayStatics.ApplyDamage` _output 5.0)
    (`KismetSystemLibrary.PrintString` (`KismetSystemLibrary.GetDisplayName` _output))))

(fn `GetSpeedCo`
  (returns (SpeedCo :type "Float (double-precision)"))
  (return 0.0))

(fn `Play Anim`
  (`SkeletalMeshComponent.PlayAnimation` (`self.Melee_Weapon`) "/Game/Dynamic/Weapons/Sword/Animation/A_Swing.A_Swing" false))

(fn `UserConstructionScript`)